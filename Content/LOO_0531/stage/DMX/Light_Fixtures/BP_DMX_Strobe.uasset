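; DMX strobe light fixture Blueprint that drives a point light and lens material from received fixture patch data.
; It initializes with the lens mesh, pushes normalized DMX attribute values to the fixture and interpolates its DMX components every tick.
; Each tick it also shows the point light only when the lens material's dimmer is above zero and the light color is not black.
; The construction script poses Yoke and Head from rotation variables.
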(event `self.ReceiveBeginPlay`
  ;[1 1 1] Init
  (`self.InitializeFixture` (`self.StaticMeshLens`)))

(event `self.ReceiveTick`
  (params (DeltaSeconds :type "Float (double-precision)"))
  ;[1 1 1] Update
  (`self.InterpolateDMXComponents` DeltaSeconds)
  (`self.ToggleLightVisibility`))

(event `self.DMX.OnFixturePatchReceived`
  (params (FixturePatch :type "Object Object Reference") (ValuePerAttribute :type " Structure (by ref)"))
  ;[1 1 1] On data received
  (`self.PushNormalizedValuesPerAttribute` ValuePerAttribute))

(fn `ToggleLightVisibility`
  (bind _dynamicmateriallens (`self.DynamicMaterialLens`))
  (if (`KismetSystemLibrary.IsValid` _dynamicmateriallens)
    (bind _returnvalue (`MaterialInstanceDynamic.K2_GetScalarParameterValue` _dynamicmateriallens "DMX Dimmer"))
    (`SceneComponent.SetVisibility` (`self.PointLight`) (and (> _returnvalue 0.0) (!= (`LightComponentBase.GetLightColor` (`self.PointLight`)) (struct))) false)))

(fn `UserConstructionScript`
  (`SceneComponent.K2_SetRelativeRotation` (`self.Yoke`) (`KismetMathLibrary.MakeRotator` (`self.Vertical_Rotation`) 0.0) false false)
  (`SceneComponent.K2_SetRelativeRotation` (`self.Head`) (`KismetMathLibrary.MakeRotator` 0.0 (`self.Horizontal_Rotation (Up and Down)`)) false false))